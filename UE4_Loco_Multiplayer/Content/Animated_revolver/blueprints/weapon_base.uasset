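; Base revolver weapon Blueprint that shows live rounds and spent shells in the barrel to match the current bullet count.
; BeginPlay stores six bullet mesh components in an ordered array and refreshes them.
; The update event sets or adds to BulletCount, then triggers the refresh.
; Refresh loops the array, assigning the shell mesh to indices at or above the count and the bullet mesh to the rest.
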(event Custom|update_bullet
  (params (set_bullets :type Integer) (add :type Boolean))
  ;[1 1 1] Here we do store bullets in the array,
  ; for revolver logic.
  (if add
    (Variables|Default|Setbullet_count (+ set_bullets (Variables|Default|Getbullet_count)))
    (else
      (Variables|Default|Setbullet_count set_bullets)))
  (CallFunction|RefreshBullet) ; refresh bullet to show correct visuals.
)

(event Custom|refresh_bullet
  ;[1 1 1] Here we do store bullets in the array,
  ; for revolver logic.
  (for (_array_element _array_index) (Variables|Default|Getbullet_list)
    (if (>= _array_index (Variables|Default|Getbullet_count)) ; we check if index\nof bullet is equal or higher\nthan bullet count,\nthis means that bullet is used\nand shold be swapped by shell.
      (Components|StaticMesh|SetStaticMesh _array_element "/Game/Animated_revolver/staticmeshes/static_shell.static_shell")
      (else
        (Components|StaticMesh|SetStaticMesh _array_element "/Game/Animated_revolver/staticmeshes/static_bullet.static_bullet") ; if we have enough bullets in barrel\nwe should show the bullet mesh.
      ))))

(event EventBeginPlay
  ;[1 1 1] Here we do store bullets in the array,
  ; for revolver logic.
  (Variables|Default|Setbullet_list (Utilities|Array|MakeArray (Variables|Default|Get1) (Variables|Default|Get2) (Variables|Default|Get3) (Variables|Default|Get4) (Variables|Default|Get5) (Variables|Default|Get6))) ; we store static bullets to array list,\nthe order of mesh and list is important.
  (CallFunction|RefreshBullet) ; refresh to show correct\namount of bullets in barrel.
)

(fn ConstructionScript)